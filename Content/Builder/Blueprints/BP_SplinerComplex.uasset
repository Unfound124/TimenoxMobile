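; BP_SplinerComplex is a builder actor that generates spline meshes along an optionally looped spline when Generate is enabled.
; The construction script adds one deformed mesh per segment, using the point tangents, up vector and a per-mesh scale.
; It then places optional Connector static meshes at each point, rotated along the tangent.
; Meshes and connectors each either cycle through their arrays or are picked randomly from a seeded stream.
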(fn `UserConstructionScript`
  (locals (RandomMesh :type Integer :default 0) (RandomConn :type Integer :default 0))
  (bind _loop (`self.Loop`))
  (bind _spline (`self.Spline`))
  (bind _returnvalue (`KismetArrayLibrary.Array_Length` (`self.Connector`)))
  (bind _returnvalue_2 (`KismetArrayLibrary.Array_Length` (`self.Mesh`)))
  (bind _returnvalue_3 (`KismetArrayLibrary.Array_Length` (`self.Connector`)))
  (bind _returnvalue_4 (`SplineComponent.GetNumberOfSplinePoints` (`self.Spline`)))
  (if (`self.Generate`)
    (`KismetArrayLibrary.Array_Resize` (`self.MeshScale`) (`KismetArrayLibrary.Array_Length` (`self.Mesh`)))
    (`SplineComponent.SetClosedLoop` (`self.Spline`) _loop true)
    (`|ExecutionSequence`
      (:`then_0`
        (for _index (range 1 (+ (`KismetMathLibrary.SelectInt` _returnvalue_4 (- _returnvalue_4 1) _loop) 1))
          (bind _output_get (set `local.RandomMesh` (`KismetMathLibrary.RandomIntegerFromStream` _returnvalue_2 (`self.Seed`))))
          (bind _returnvalue_5 (`AddComponent|NODE_AddSplineMeshComponent-0`))
          (bind _returnvalue_6 (- _index 1))
          (bind _returnvalue_7 (select `/Game/Builder/Blueprints/ESelect` (`self.MeshSelection`) :`NewEnumerator0` (mod _returnvalue_6 _returnvalue_2) :`NewEnumerator1` _output_get))
          (`StaticMeshComponent.SetStaticMesh` _returnvalue_5 (`|GetArrayItem` (`self.Mesh`) _returnvalue_7))
          (bind (_location _tangent) (`SplineComponent.GetLocationAndTangentAtSplinePoint` _spline _returnvalue_6 "Local"))
          (bind (_location_2 _tangent_2) (`SplineComponent.GetLocationAndTangentAtSplinePoint` _spline _index "Local"))
          (`SplineMeshComponent.SetStartAndEnd` _returnvalue_5 _location _tangent _location_2 _tangent_2 true)
          (`SplineMeshComponent.SetForwardAxis` _returnvalue_5 (`self.MeshForwardVector`) true)
          (`SplineMeshComponent.SetSplineUpDir` _returnvalue_5 (`SplineComponent.GetUpVectorAtSplinePoint` _spline _index "Local") true)
          (bind _output (`|GetArrayItem` (`self.MeshScale`) _returnvalue_7))
          (`SplineMeshComponent.SetStartScale` _returnvalue_5 _output true)
          (`SplineMeshComponent.SetEndScale` _returnvalue_5 _output true)))
      (:`then_1`
        (if (> _returnvalue_3 0)
          (`KismetArrayLibrary.Array_Resize` (`self.ConnectorScale`) _returnvalue_3)
          (for _index_2 (range (`SplineComponent.GetNumberOfSplinePoints` (`self.Spline`)))
            (set `local.RandomConn` (`KismetMathLibrary.RandomIntegerFromStream` _returnvalue (`self.Seed`)))
            (bind (_location_3 _tangent_3) (`SplineComponent.GetLocationAndTangentAtSplinePoint` (`self.Spline`) _index_2 "Local"))
            (bind _returnvalue_8 (select `/Game/Builder/Blueprints/ESelect` (`self.ConnectorSelection`) :`NewEnumerator0` (mod _index_2 _returnvalue) :`NewEnumerator1` (`local.RandomConn`)))
            (bind _returnvalue_9 (`AddComponent|NODE_AddStaticMeshComponent-0` :`RelativeTransform` (`KismetMathLibrary.MakeTransform` _location_3 (`KismetMathLibrary.Conv_VectorToRotator` _tangent_3) (`|GetArrayItem` (`self.ConnectorScale`) _returnvalue_8))))
            (`StaticMeshComponent.SetStaticMesh` _returnvalue_9 (`|GetArrayItem` (`self.Connector`) _returnvalue_8))))))))