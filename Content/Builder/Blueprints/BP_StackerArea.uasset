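; BP_StackerArea is a construction-script scatter tool that fills an area around the actor with instances of one mesh when Generate is on.
; Each instance gets a randomized horizontal offset, with Ratio shaping how distance spreads up to Radius.
; With TraceDown, line traces drop instances onto surfaces, optionally normal-aligned, with random location, rotation and scale variation.
; Otherwise, instances float at random heights up to Height using the base rotation and scale.
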(fn `UserConstructionScript`
  (bind _returnvalue (`KismetMathLibrary.RandomFloatInRange` 0.0 360.0))
  (bind _returnvalue_2 (`KismetMathLibrary.RandomFloatInRange` 0.0 360.0))
  (bind _amount (`self.Amount`))
  (if (`self.Generate`)
    (`StaticMeshComponent.SetStaticMesh` (`self.InstancedStaticMesh`) (`self.Mesh`))
    (for _index (range _amount)
      (if (`self.TraceDown`)
        (bind _returnvalue_3 (* (`KismetMathLibrary.MultiplyMultiply_FloatFloat` (/ (`KismetMathLibrary.Conv_IntToDouble` (+ _index 1)) (`KismetMathLibrary.Conv_IntToDouble` _amount)) (`self.Ratio`)) (`self.Radius`)))
        (bind _returnvalue_4 (+ (`self.K2_GetActorLocation`) (* (`KismetMathLibrary.MakeVector` (`KismetMathLibrary.DegCos` _returnvalue_2) (`KismetMathLibrary.DegSin` _returnvalue_2)) _returnvalue_3)))
        (bind _outhit (`KismetSystemLibrary.LineTraceSingleForObjects` _returnvalue_4 (+ _returnvalue_4 (* (`self.GetActorUpVector`) -65535.0)) (`self.TraceTypes`)))
        (bind (_bblockinghit _binitialoverlap _time _distance _location _impactpoint _normal _impactnormal) (`GameplayStatics.BreakHitResult` _outhit))
        (`InstancedStaticMeshComponent.AddInstanceWorldSpace` (`self.InstancedStaticMesh`) (`/Game/Builder/Blueprints/BP_FuncLib.CombineTransform` (`KismetMathLibrary.MakeTransform` (`/Game/Builder/Blueprints/BP_FuncLib.RandomVector` (`self.MinRandomLocation`) (`self.MaxRandomLocation`)) (`/Game/Builder/Blueprints/BP_FuncLib.RandomRot` (`self.MinRandomRotation`) (`self.MaxRandomRotation`)) (`/Game/Builder/Blueprints/BP_FuncLib.RandomVector` (`self.MinRandomScale`) (`self.MaxRandomScale`))) (`KismetMathLibrary.MakeTransform` (+ (* _impactnormal (`self.Height`)) _impactpoint) (`KismetMathLibrary.SelectRotator` (`KismetMathLibrary.MakeRotFromZ` _impactnormal) (`self.BaseRotation`) (`self.UseNormal`)) (`self.BaseScale`))))
        (else
          (`InstancedStaticMeshComponent.AddInstance` (`self.InstancedStaticMesh`) (`KismetMathLibrary.MakeTransform` (+ (* (`KismetMathLibrary.MakeVector` (`KismetMathLibrary.DegCos` _returnvalue) (`KismetMathLibrary.DegSin` _returnvalue)) _returnvalue_3) (`KismetMathLibrary.MakeVector` 0.0 0.0 (`KismetMathLibrary.RandomFloatInRange` 0.0 (`self.Height`)))) (`self.BaseRotation`) (`self.BaseScale`))))))))