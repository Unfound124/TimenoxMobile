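; Function library of overlap queries that the dungeon generator uses to find DungeonTile neighbors.
; GetConnectedTiles maps each connection component to its first overlapping tile, keeping empty entries so indices stay aligned, while GetOverlappingTiles gathers every unique overlapping tile, both ignoring the component's owner.
; CheckTilesForRows flags tiles whose data table row is in a given list.
; GetSingleOverlappingTile combines the latter two to return the first overlapping tile with a matching row.
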(fn `CheckTilesForRows`
  (params (Tiles :type "Array of /Game/DungeonGenerator/Blueprints/DungeonTile Object Reference") (Rows :type "Array of Name"))
  (returns (Return :type "Array of Boolean"))
  (locals (Matches :type "Array of Boolean"))
  (for _array_element Tiles
    (`/Engine/EditorBlueprintResources/StandardMacros.IsValid` _array_element
      (:`Is Valid`
        (`KismetArrayLibrary.Array_Add` (`local.Matches`) (`KismetArrayLibrary.Array_Contains` (`local.Rows`) (`/Game/DungeonGenerator/Blueprints/DungeonTile.DataTableRow` _array_element))))
      (:`Is Not Valid`
        (`KismetArrayLibrary.Array_Add` (`local.Matches`)))))
  (return (`local.Matches`)))

(fn `GetConnectedTiles`
  (params (Connections :type "Array of BoxComponent Object Reference"))
  (returns (Tiles :type "Array of /Game/DungeonGenerator/Blueprints/DungeonTile Object Reference"))
  (locals (ConnectionBoxes :type "Array of /Game/DungeonGenerator/Blueprints/DungeonTile Object Reference"))
  (bind _connectionboxes (`local.ConnectionBoxes`))
  (for _array_element Connections
    (bind (_outactors _returnvalue) (`KismetSystemLibrary.ComponentOverlapActors` _array_element (`SceneComponent.K2_GetComponentToWorld` _array_element) (`|MakeArray` "ObjectTypeQuery6" "ObjectTypeQuery1" :!type "EObjectTypeQuery Enum") "/Game/DungeonGenerator/Blueprints/DungeonTile.DungeonTile_C" (`|MakeArray` (`ActorComponent.GetOwner` _array_element))))
    (if _returnvalue
      (`KismetArrayLibrary.Array_Add` _connectionboxes (cast `/Game/DungeonGenerator/Blueprints/DungeonTile` (`|GetArrayItem` _outactors) :!pure true))
      (else
        (`KismetArrayLibrary.Array_Add` _connectionboxes))))
  (return (`local.ConnectionBoxes`)))

(fn `GetOverlappingTiles`
  (params (Component :type "PrimitiveComponent Object Reference"))
  (returns (Return :type Boolean) (Tiles :type "Array of /Game/DungeonGenerator/Blueprints/DungeonTile Object Reference"))
  (locals (DungeonTiles :type "Array of /Game/DungeonGenerator/Blueprints/DungeonTile Object Reference"))
  (bind (_outactors _returnvalue) (`KismetSystemLibrary.ComponentOverlapActors` Component (`SceneComponent.K2_GetComponentToWorld` Component) (`|MakeArray` "ObjectTypeQuery1" "ObjectTypeQuery6" :!type "EObjectTypeQuery Enum") "/Game/DungeonGenerator/Blueprints/DungeonTile.DungeonTile_C" (`|MakeArray` (`ActorComponent.GetOwner` Component))))
  (for _array_element _outactors
    (bind _asdungeon_tile (cast `/Game/DungeonGenerator/Blueprints/DungeonTile` _array_element))
    (`KismetArrayLibrary.Array_AddUnique` (`local.DungeonTiles`) _asdungeon_tile))
  (return _returnvalue (`local.DungeonTiles`)))

(fn `GetSingleOverlappingTile`
  (params (Component :type "PrimitiveComponent Object Reference") (Rows :type "Array of Name (by ref)"))
  (returns (Tile :type "/Game/DungeonGenerator/Blueprints/DungeonTile Object Reference"))
  (bind (_return _tiles) (`self.GetOverlappingTiles` Component Component))
  (if _return
    (bind _return_2 (`self.CheckTilesForRows` _tiles (`local.Rows`) (`local.Component`)))
    (bind _returnvalue (`KismetArrayLibrary.Array_Find` _return_2 true))
    (if (!= _returnvalue -1)
      (return (`|GetArrayItem` _tiles _returnvalue))
      (else
        (return null)))
    (else
      (return null))))