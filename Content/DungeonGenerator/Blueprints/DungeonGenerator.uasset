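; Dungeon generator actor that builds a random tile layout at BeginPlay, growing from placed tiles' connections behind an optional loading screen.
; Weighted, amount-limited DataTable rows spawn onto random or center-nearest connections, aligned via Arrow attachment and validated.
; Ticks are spread across frames, switching to brute force when stalled.
; Layouts below the required size restart; others get dead ends, modifiers and interface notifications, with meshes batched into material-matched HISMs.
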(event `Restart`
  (bind _returnvalue (`KismetArrayLibrary.Array_Length` (`self.UnfinishedConnections`)))
  (`self.SetupGenerator` :!label _label)
  (`LowEntryExtendedStandardLibrary.DelayFrames` 1)
  (`self.GetExistingTileConnections`)
  (`self.CreateTilePool`)
  (if (not (or (>= (`self.LayoutTilesSpawned`) (`self.TileAmountTarget`)) (== _returnvalue 0) (<= _returnvalue (`KismetArrayLibrary.Array_Length` (`self.ConnectionBlacklist`))))) :!label _label_2
    (bind _outactors (`GameplayStatics.GetAllActorsOfClass` "/Game/DungeonGenerator/Blueprints/DungeonTile.DungeonTile_C"))
    (if (== (`KismetArrayLibrary.Array_Length` _outactors) (`self.LastTileAmount`))
      (bind _result (`/Engine/EditorBlueprintResources/StandardMacros.IncrementInt` (`self.RetryCounter`))
        (:`  `
          (if (>= _result (`self.TicksBeforeBruteForceMode`))
            (`/Engine/EditorBlueprintResources/StandardMacros.FlipFlop`
              (:`A`
                (`self.MinimizeTilePool`)
                (set `self.RetryCounter` 0)
                (bind _outactors_2 (`GameplayStatics.GetAllActorsOfClass` "/Game/DungeonGenerator/Blueprints/DungeonTile.DungeonTile_C" :!label _label_3))
                (set `self.LastTileAmount` (`KismetArrayLibrary.Array_Length` _outactors_2))
                (`self.AddTileToConnection`)
                (bind _result_2 (`/Engine/EditorBlueprintResources/StandardMacros.IncrementInt` (`self.TickCounter`))
                  (:`  `
                    (if (>= _result_2 (select `bool` (`self.IsBruteForceMode`) :`false` (`self.TicksPerFrame`) :`true` (`KismetMathLibrary.FCeil` (/ (`KismetMathLibrary.Conv_IntToDouble` (`self.TicksPerFrame`)) 5.0))))
                      (`LowEntryExtendedStandardLibrary.DelayFrames` 1)
                      (set `self.TickCounter` 0)
                      (goto _label_2)
                      (else
                        (goto _label_2))))))
              (:`B`
                _))
            (else
              (goto _label_3)))))
      (else
        (set `self.RetryCounter` 0)
        (goto _label_3))))
  (bind _return (`self.AfterLayout`))
  (if _return
    (if (>= (`self.TilesSpawned`) (`self.LayoutTilesSpawned`)) :!label _label_4
      (`self.AfterSpawning`)
      (else
        (`LowEntryExtendedStandardLibrary.DelayFrames` 1)
        (goto _label_4)))
    (else
      (`self.RestartGenerator`))))

(event `self.ReceiveBeginPlay`
  (goto _label))

(fn `AddInstancedMesh`
  (params (Mesh :type "StaticMeshComponent Object Reference"))
  (locals (ComponentFound :type Boolean) (FoundEntry :type "/Game/DungeonGenerator/Data/InstancedMeshEntry Structure"))
  (bind (_value _returnvalue) (`BlueprintMapLibrary.Map_Find` (`self.InstancedMeshes`) (`StaticMeshComponent.StaticMesh` Mesh)))
  (if _returnvalue
    (bind _output_get (set `local.FoundEntry` _value))
    (bind _return (`self.FindInstancedMeshComponent` _output_get (`local.Mesh`)))
    (if _return
      (`self.K2_AddActorWorldOffset` (0.0 0.0 1.0))
      (`self.K2_AddActorWorldOffset` (0.0 0.0 -1.0))
      (return)
      (else
        (`self.AddNewInstancedMeshToEntry` (`local.FoundEntry`) (`local.Mesh`))
        (return)))
    (else
      (`self.AddNewInstancedMeshToEntry` (make `/Game/DungeonGenerator/Data/InstancedMeshEntry` (`|MakeArray`)) (`local.Mesh`))
      (return))))

(fn `AddNewInstancedMeshToEntry`
  (params (Entry :type "/Game/DungeonGenerator/Data/InstancedMeshEntry Structure (by ref)") (Mesh :type "StaticMeshComponent Object Reference"))
  (bind _entries (break `/Game/DungeonGenerator/Data/InstancedMeshEntry` (`local.Entry`)))
  (bind _returnvalue (`self.CreateInstancedMeshComponent` Mesh))
  (`KismetArrayLibrary.Array_Add` _entries (make `/Game/DungeonGenerator/Data/InstancedMeshMaterialEntry` (`MeshComponent.GetMaterials` Mesh) _returnvalue))
  (`BlueprintMapLibrary.Map_Add` (`self.InstancedMeshes`) (`StaticMeshComponent.StaticMesh` (`local.Mesh`)) (make `/Game/DungeonGenerator/Data/InstancedMeshEntry` _entries))
  (`self.AddInstancedMesh` (`local.Mesh`))
  (return))

(fn `AddTileToConnection`
  (locals (Connection :type "BoxComponent Object Reference"))
  (bind _connection (`local.Connection`))
  (if (`self.UseFromCenterMode`)
    (bind _connection_2 (`self.SelectConnectionByDistance`))
    (set `local.Connection` _connection_2)
    (else
      (set `local.Connection` (`self.SelectRandomBoxComponent` (`self.UnfinishedConnections`)))))
  (if (`self.IsBruteForceMode`)
    (`self.BruteForceMode` _connection)
    (return)
    (else
      (`self.RandomSpawn` _connection)
      (return))))

(fn `AfterLayout`
  (returns (Return :type Boolean))
  (bind _outactors (`GameplayStatics.GetAllActorsOfClass` "/Game/DungeonGenerator/Blueprints/DungeonTile.DungeonTile_C"))
  (if (>= (`KismetArrayLibrary.Array_Length` _outactors) (`self.TileAmountRequired`))
    (`self.SpawnDeadEnds`)
    (`KismetArrayLibrary.Array_Clear` (`self.UnfinishedConnections`))
    (bind _outactors_2 (`GameplayStatics.GetAllActorsOfClass` "/Game/DungeonGenerator/Blueprints/LayoutModifier.LayoutModifier_C"))
    (`/Game/DungeonGenerator/Blueprints/LayoutModifier.ModifyLayout` _outactors_2)
    (bind _outactors_3 (`GameplayStatics.GetAllActorsWithInterface` "/Game/DungeonGenerator/Blueprints/DungeonInterface.DungeonInterface_C"))
    (for _array_element _outactors_3
      (`/Engine/EditorBlueprintResources/StandardMacros.IsValid` _array_element
        (:`Is Valid`
          (message `/Game/DungeonGenerator/Blueprints/DungeonInterface.LayoutFinished` _array_element self))))
    (set `/Game/DungeonGenerator/LoadingScreen.UpdateOnTick` true (`self.LoadingWidget`))
    (return true)
    (else
      (return false))))

(fn `AfterSpawning`
  (`/Engine/EditorBlueprintResources/StandardMacros.IsValid` (`self.LoadingWidget`)
    (:`Is Valid`
      (`Widget.RemoveFromParent` (`self.LoadingWidget`)))
    (:`Is Not Valid`
      _))
  (bind _outactors (`GameplayStatics.GetAllActorsWithInterface` "/Game/DungeonGenerator/Blueprints/DungeonInterface.DungeonInterface_C"))
  (message `/Game/DungeonGenerator/Blueprints/DungeonInterface.SpawningFinished` _outactors self)
  (bind _outactors_2 (`GameplayStatics.GetAllActorsOfClass` "/Game/DungeonGenerator/Blueprints/LayoutModifier.LayoutModifier_C"))
  (`self.K2_DestroyActor` _outactors_2)
  (`self.CheckMaterialCompability`))

(fn `BruteForceMode`
  (params (Connection :type "BoxComponent Object Reference"))
  (locals (ShuffledTiles :type "Array of Name"))
  (bind _output_get (set `local.ShuffledTiles` (`self.TilePool`)))
  (`KismetArrayLibrary.Array_Shuffle` _output_get)
  (for _array_element (`local.ShuffledTiles`)
    (bind _return (`self.CreateTile` _array_element (`self.GetConnection` (`local.Connection`)) (`self.SnapTransform` (`SceneComponent.K2_GetComponentToWorld` (`local.Connection`)))))
    (if _return
      (break)))
  (return))

(fn `CheckInstanceMaterials`
  (params (Materials :type "Array of MaterialInterface Object Reference") (Mesh :type "StaticMeshComponent Object Reference"))
  (returns (Return :type Boolean))
  (locals (MaterialsMatch :type Boolean :default true))
  (for (_array_element _array_index) Materials
    (if (not (== _array_element (`|GetArrayItem` (`MeshComponent.GetMaterials` Mesh) _array_index)))
      (set `local.MaterialsMatch` false)
      (break)))
  (return (`local.MaterialsMatch`)))

(fn `CheckMaterialCompability`
  (locals (IncompatibleMaterials :type "Array of Material Object Reference"))
  (bind _values (`BlueprintMapLibrary.Map_Values` (`self.InstancedMeshes`)))
  (for _array_element _values
    (for _array_element_2 (`.Entries_3_7368235F4E486DF9B88A3989B9F03B6A` (break `/Game/DungeonGenerator/Data/InstancedMeshEntry` _array_element))
      (for _array_element_3 (`MeshComponent.GetMaterials` (`.Component_6_8A9AEEDD47F89080DF4BACBCE49E67E8` (break `/Game/DungeonGenerator/Data/InstancedMeshMaterialEntry` _array_element_2)))
        (bind _returnvalue (`MaterialInterface.GetBaseMaterial` _array_element_3))
        (if (not (`Material.bUsedWithInstancedStaticMeshes` _returnvalue))
          (`KismetArrayLibrary.Array_AddUnique` (`local.IncompatibleMaterials`) _returnvalue)))))
  (for _array_element_4 (`local.IncompatibleMaterials`)
    (`KismetSystemLibrary.PrintString` (`KismetStringLibrary.Concat_StrStr` "Material \"" (`KismetSystemLibrary.GetDisplayName` _array_element_4) "\" cannot be used with instanced static meshes. \nMake it compatible by checking the correct checkbox \nin it's properties.") true true (struct :`R` 1.0 :`A` 1.0) 20.0))
  (return))

(fn `ContainsMatchingConnection`
  (params (RowName :type Name) (Connection :type Name))
  (returns (Return :type Boolean) (MatchingConnection :type "/Game/DungeonGenerator/Data/TileConnection Structure"))
  (locals (ContainsConnection :type Boolean) (FoundConnection :type "/Game/DungeonGenerator/Data/TileConnection Structure") (Connections :type "Array of /Game/DungeonGenerator/Data/TileConnection Structure"))
  (bind _returnvalue (`|GetDataTableRow` (`self.Tiles`) RowName)
    (:`then`
      (bind _output_get (set `local.Connections` (`.Connections_6_45BF8D50405223D2E59948B062AA2031` (break `/Game/DungeonGenerator/Data/TileData` (`.TileData_3_9898053E4AEB04A7AD36ACA2E4DA45FC` (break `/Game/DungeonGenerator/Data/TileEntry` _returnvalue))))))
      (`KismetArrayLibrary.Array_Shuffle` _output_get)
      (for _array_element _output_get
        (bind ((`Type_7_26122FC74EFF9E7F8E9B71B59A37741A` _type) (`DontStartHere_9_FC4EB5564C7BFFB55BE445BA34D09BE6` _dontstarthere)) (break `/Game/DungeonGenerator/Data/TileConnection` _array_element))
        (if (not _dontstarthere)
          (bind _returnvalue_2 (`|GetDataTableRow` (`self.ConnectionMatches`) (`local.Connection`))
            (:`then`
              (if (`KismetArrayLibrary.Array_Contains` (`.MatchesWith_6_8802C2754F8795C67A4F4D9AE7154197` (break `/Game/DungeonGenerator/Data/ConnectionMatch` _returnvalue_2)) _type)
                (set `local.ContainsConnection` true)
                (set `local.FoundConnection` _array_element)
                (break))))))
      (return (`local.ContainsConnection`) (`local.FoundConnection`)))
    (:`RowNotFound`
      (return false))))

(fn `CreateInstancedMeshComponent`
  (params (Mesh :type "StaticMeshComponent Object Reference"))
  (returns (ReturnValue :type "HierarchicalInstancedStaticMeshComponent Object Reference"))
  (bind _returnvalue (`AddComponent|NODE_AddHierarchicalInstancedStaticMeshComponent-0`))
  (`StaticMeshComponent.SetStaticMesh` _returnvalue (`StaticMeshComponent.StaticMesh` Mesh))
  (for (_array_element _array_index) (`MeshComponent.GetMaterials` Mesh)
    (`PrimitiveComponent.SetMaterial` _returnvalue _array_index _array_element))
  (return _returnvalue))

(fn `CreateTile`
  (params (RowName :type Name) (Connection :type Name) (Transform :type "Transform Structure") (SkipChecks :type Boolean))
  (returns (Return :type Boolean) (Tile :type "/Game/DungeonGenerator/Blueprints/DungeonTile Object Reference"))
  (locals (SpawnedTile :type "/Game/DungeonGenerator/Blueprints/DungeonTile Object Reference"))
  (bind _spawnedtile (`local.SpawnedTile`))
  (bind (_return _matchingconnection) (`self.ContainsMatchingConnection` RowName Connection))
  (if _return
    (bind _returnvalue (`|SpawnActorFromClass` "/Game/DungeonGenerator/Blueprints/DungeonTile.DungeonTile_C" (`KismetMathLibrary.MakeTransform` (0.0 0.0 0.0)) "AlwaysSpawn" "OverrideRootScale" null (`local.RowName`) self null))
    (set `local.SpawnedTile` _returnvalue)
    (`SceneComponent.K2_SetWorldTransform` (`self.Arrow`) (`self.SnapTransform` (`.Transform_2_C1FF5E8344E708A538E5D9ADCC5696B7` (break `/Game/DungeonGenerator/Data/TileConnection` _matchingconnection))) false false)
    (`SceneComponent.K2_AddLocalRotation` (`self.Arrow`) (struct :`Yaw` 180.0) false false)
    (`self.K2_AttachToComponent` (`local.SpawnedTile`) (`self.Arrow`) "None" "KeepWorld" "KeepWorld" "KeepWorld" true)
    (`SceneComponent.K2_SetWorldTransform` (`self.Arrow`) (`local.Transform`) false false)
    (`self.K2_DetachFromActor` (`local.SpawnedTile`) "KeepWorld" "KeepWorld" "KeepWorld")
    (bind _return_2 (`/Game/DungeonGenerator/Blueprints/DungeonTile.RunChecks` (`local.SpawnedTile`) (`local.SkipChecks`)))
    (if _return_2
      (`self.FinishTile` _spawnedtile)
      (return true (`local.SpawnedTile`))
      (else
        (`/Game/DungeonGenerator/Blueprints/DungeonTile.DestroyTile` _spawnedtile false)
        (return false null)))
    (else
      (return false null))))

(fn `CreateTilePool`
  (bind _outrownames (`DataTableFunctionLibrary.GetDataTableRowNames` (`self.Tiles`)))
  (for _array_element _outrownames
    (bind _returnvalue (`|GetDataTableRow` (`self.Tiles`) _array_element)
      (:`then`
        (bind ((`Amount_18_EBA166B04461E261D737BF8C6BD3E1F0` _amount) (`Probability_16_5E4B51C54F4183FC375562AC7847BBAA` _probability)) (break `/Game/DungeonGenerator/Data/TileData` (`.TileData_3_9898053E4AEB04A7AD36ACA2E4DA45FC` (break `/Game/DungeonGenerator/Data/TileEntry` _returnvalue))))
        (if (>= _probability 1)
          (for _ (range 1 (+ _probability 1))
            (`KismetArrayLibrary.Array_Add` (`self.TilePool`) _array_element))
          (if (> _amount 0)
            (`BlueprintMapLibrary.Map_Add` (`self.RowAmounts`) _array_element _amount))))))
  (return))

(fn `FindInstancedMeshComponent`
  (params (InstancedMeshList :type "/Game/DungeonGenerator/Data/InstancedMeshEntry Structure") (Mesh :type "StaticMeshComponent Object Reference"))
  (returns (Return :type Boolean))
  (locals (ComponentFound :type Boolean))
  (for _array_element (`.Entries_3_7368235F4E486DF9B88A3989B9F03B6A` (break `/Game/DungeonGenerator/Data/InstancedMeshEntry` InstancedMeshList))
    (bind (_materials _component) (break `/Game/DungeonGenerator/Data/InstancedMeshMaterialEntry` _array_element))
    (bind _return (`self.CheckInstanceMaterials` _materials (`local.Mesh`)))
    (if _return
      (`InstancedStaticMeshComponent.AddInstanceWorldSpace` _component (`SceneComponent.K2_GetComponentToWorld` (`local.Mesh`)))
      (set `local.ComponentFound` true)
      (break)))
  (return (`local.ComponentFound`)))

(fn `FinishTile`
  (params (Tile :type "/Game/DungeonGenerator/Blueprints/DungeonTile Object Reference"))
  (bind _tile (`local.Tile`))
  (`self.RemoveRowAmount` (`/Game/DungeonGenerator/Blueprints/DungeonTile.DataTableRow` Tile))
  (`/Engine/EditorBlueprintResources/StandardMacros.IncrementInt` (`self.LayoutTilesSpawned`)
    (:`  `
      (`/Game/DungeonGenerator/Blueprints/DungeonTile.SpawnModifier` _tile)
      (for _array_element (`/Game/DungeonGenerator/Blueprints/DungeonTile.ConnectionsToRemove` _tile)
        (`KismetArrayLibrary.Array_RemoveItem` (`self.UnfinishedConnections`) _array_element))
      (return))))

(fn `GetExistingTileConnections`
  (`KismetArrayLibrary.Array_Clear` (`self.UnfinishedConnections`))
  (bind _outactors (`GameplayStatics.GetAllActorsOfClass` "/Game/DungeonGenerator/Blueprints/DungeonTile.DungeonTile_C"))
  (bind _output_get (set `self.KeepTilesAfterRestart` _outactors))
  (for _array_element _output_get
    (for _array_element_2 (`/Game/DungeonGenerator/Blueprints/DungeonTile.Connections` _array_element)
      (`KismetArrayLibrary.Array_AddUnique` (`self.UnfinishedConnections`) _array_element_2))
    (`self.FinishTile` _array_element))
  (return))

(fn `MinimizeTilePool`
  (locals (RemoveIndices :type "Array of Integer"))
  (for (_array_element _array_index) (`self.TilePool`)
    (if (< (`KismetArrayLibrary.Array_Find` (`self.TilePool`) _array_element) _array_index)
      (`KismetArrayLibrary.Array_Add` (`local.RemoveIndices`) _array_index)))
  (for (_array_element_2 _array_index_2) (`local.RemoveIndices`)
    (`KismetArrayLibrary.Array_Remove` (`self.TilePool`) (- _array_element_2 _array_index_2)))
  (set `self.IsBruteForceMode` true)
  (return))

(fn `RandomSpawn`
  (params (Connection :type "BoxComponent Object Reference"))
  (`self.CreateTile` (`self.SelectRandomName` (`self.TilePool`)) (`self.GetConnection` Connection) (`self.SnapTransform` (`SceneComponent.K2_GetComponentToWorld` Connection)))
  (return))

(fn `RemoveRowAmount`
  (params (Key :type Name))
  (bind (_value _returnvalue) (`BlueprintMapLibrary.Map_Find` (`self.RowAmounts`) Key))
  (if _returnvalue
    (`BlueprintMapLibrary.Map_Add` (`self.RowAmounts`) (`local.Key`) (- _value 1))
    (if (<= _value 0)
      (`KismetArrayLibrary.Array_RemoveItem` (`self.TilePool`) (`local.Key`))
      (return)
      (else
        (return)))
    (else
      (return))))

(fn `RestartGenerator`
  (bind _outactors (`GameplayStatics.GetAllActorsOfClass` "/Game/DungeonGenerator/Blueprints/DungeonTile.DungeonTile_C"))
  (for _array_element _outactors
    (if (not (`KismetArrayLibrary.Array_Contains` (`self.KeepTilesAfterRestart`) _array_element))
      (`self.K2_DestroyActor` _array_element)))
  (set `self.LayoutTilesSpawned` 0)
  (set `self.TilesSpawned` 0)
  (`KismetArrayLibrary.Array_Clear` (`self.TilePool`))
  (`BlueprintMapLibrary.Map_Clear` (`self.RowAmounts`))
  (`KismetArrayLibrary.Array_Clear` (`self.UnfinishedConnections`))
  (set `self.LastTileAmount` 0)
  (set `self.RetryCounter` 0)
  (set `self.TickCounter` 0)
  (`BlueprintMapLibrary.Map_Clear` (`self.InstancedMeshes`))
  (set `self.IsBruteForceMode` false)
  (`/Engine/EditorBlueprintResources/StandardMacros.IsValid` (`self.LoadingWidget`)
    (:`Is Valid`
      (`Widget.RemoveFromParent` (`self.LoadingWidget`)))
    (:`Is Not Valid`
      _))
  (`self.Restart`)
  (return))

(fn `SelectConnectionByDistance`
  (returns (Connection :type "BoxComponent Object Reference"))
  (locals (Distances :type "Map of BoxComponent Object Reference to Float (double-precision)") (FoundConnection :type "BoxComponent Object Reference"))
  (for _array_element (`self.UnfinishedConnections`)
    (if (not (`KismetArrayLibrary.Array_Contains` (`self.ConnectionBlacklist`) _array_element))
      (`BlueprintMapLibrary.Map_Add` (`local.Distances`) _array_element (`KismetMathLibrary.VSize` (`SceneComponent.K2_GetComponentLocation` _array_element)))))
  (bind _values (`BlueprintMapLibrary.Map_Values` (`local.Distances`)))
  (bind _keys (`BlueprintMapLibrary.Map_Keys` (`local.Distances`)))
  (set `local.FoundConnection` (`|GetArrayItem` _keys (`KismetMathLibrary.MinOfFloatArray` _values)))
  (`|ExecutionSequence`
    (:`then_0`
      (if (== (`local.FoundConnection`) (`self.PreviousConnection`))
        (bind _result (`/Engine/EditorBlueprintResources/StandardMacros.IncrementInt` (`self.FromCenterRepeatCounter`))
          (:`  `
            (if (>= _result (`self.FromCenterModeRepeatLimit`))
              (`KismetArrayLibrary.Array_AddUnique` (`self.ConnectionBlacklist`) (`local.FoundConnection`))
              (set `self.FromCenterRepeatCounter` 0))))
        (else
          (set `self.FromCenterRepeatCounter` 0))))
    (:`then_1`
      (bind _output_get (set `self.PreviousConnection` (`local.FoundConnection`)))
      (return _output_get))))

(fn `SetupGenerator`
  (bind _returnvalue (`|CreateWidget` "/Game/DungeonGenerator/LoadingScreen.LoadingScreen_C" null self))
  (set `self.LoadingWidget` _returnvalue)
  (if (`self.ShowLoadingWidget`)
    (`UserWidget.AddToViewport` (`self.LoadingWidget`) 0)))

(fn `SpawnDeadEnds`
  (locals (NewLocalVar_0 :type Integer))
  (for _array_element (`self.UnfinishedConnections`)
    (bind _connection (`self.GetConnection` _array_element))
    (bind (_value _returnvalue) (`BlueprintMapLibrary.Map_Find` (`self.Dead-Ends`) _connection))
    (if _returnvalue
      (bind (_returnvalue_location _returnvalue_rotation) (`KismetMathLibrary.BreakTransform` (`SceneComponent.K2_GetComponentToWorld` _array_element)))
      (`self.CreateTile` _value _connection (`KismetMathLibrary.MakeTransform` _returnvalue_location _returnvalue_rotation) true)))
  (return))

(fn `UserConstructionScript`)