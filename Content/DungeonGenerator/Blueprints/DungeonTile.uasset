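; DungeonTile is a layout placeholder actor representing one piece that the DungeonGenerator places while building a dungeon.
; A data table row supplies its collision mesh, tagged connection boxes, level map and optional layout modifier and condition actors.
; Placement checks test mesh overlap, connection-type matches against a lookup table, and the condition.
; After layout it loads its map as a level instance, counts it once visible, and self-destroys when spawning finishes.
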(event `/Game/DungeonGenerator/Blueprints/DungeonInterface.SpawningFinished`
  (params (DungeonGenerator :type "/Game/DungeonGenerator/Blueprints/DungeonGenerator Object Reference"))
  (`self.K2_DestroyActor`))

(event `/Game/DungeonGenerator/Blueprints/DungeonInterface.LayoutFinished`
  (params (DungeonGenerator :type "/Game/DungeonGenerator/Blueprints/DungeonGenerator Object Reference"))
  (bind _level (`self.SpawnAssociatedLevel`))
  (`/Engine/EditorBlueprintResources/StandardMacros.IsValid` _level
    (:`Is Valid`
      (if (and (`LevelStreaming.IsLevelLoaded` _level) (`LevelStreaming.IsLevelVisible` _level)) :!label _label
        (`/Engine/EditorBlueprintResources/StandardMacros.IncrementInt` (`/Game/DungeonGenerator/Blueprints/DungeonGenerator.TilesSpawned` (`self.DungeonGenerator`)))
        (else
          (`LowEntryExtendedStandardLibrary.DelayFrames` 1)
          (goto _label))))))

(fn `CheckCollision`
  (returns (IsClear :type Boolean))
  (locals (IsOverlapping :type Boolean))
  (bind _collisionmesh (`self.CollisionMesh`))
  (`/Engine/EditorBlueprintResources/StandardMacros.IsValid` (`StaticMeshComponent.StaticMesh` _collisionmesh)
    (:`Is Valid`
      (bind (_outcomponents _returnvalue) (`KismetSystemLibrary.ComponentOverlapComponents` (`self.CollisionMesh`) (`SceneComponent.K2_GetComponentToWorld` _collisionmesh) (`|MakeArray` "ObjectTypeQuery1" :!type "EObjectTypeQuery Enum") "/Script/Engine.PrimitiveComponent" (`|MakeArray` self :!type "Actor Object Reference")))
      (return (not _returnvalue)))
    (:`Is Not Valid`
      (return true))))

(fn `CheckConnections`
  (returns (Return :type Boolean))
  (locals (ConnectionsMatch :type Boolean :default true) (RemoveFromArray :type "Array of BoxComponent Object Reference"))
  (for _array_element (`self.Connections`) :!label _label
    (for _array_element_2 (`PrimitiveComponent.GetOverlappingComponents` _array_element)
      (bind _asbox_collision (cast `BoxComponent` _array_element_2))
      (bind _return (`self.CheckSingleConnection` _asbox_collision (`|GetArrayItem` (`ActorComponent.ComponentTags` _array_element))))
      (if _return
        (`KismetArrayLibrary.Array_AddUnique` (`self.ConnectionsToRemove`) _asbox_collision)
        (`KismetArrayLibrary.Array_AddUnique` (`self.ConnectionsToRemove`) _array_element)
        (else
          (set `local.ConnectionsMatch` false)
          (goto _label :!via `Break`)))))
  (return (`local.ConnectionsMatch`)))

(fn `CheckSingleConnection`
  (params (BoxComponent :type "BoxComponent Object Reference") (Connection :type Name))
  (returns (Return :type Boolean))
  (bind _componenttags (`ActorComponent.ComponentTags` BoxComponent))
  (if (and (`KismetArrayLibrary.Array_IsValidIndex` _componenttags) (!= (`ActorComponent.GetOwner` BoxComponent) self))
    (bind _returnvalue (`|GetDataTableRow` (`/Game/DungeonGenerator/Blueprints/DungeonGenerator.ConnectionMatches` (`self.DungeonGenerator`)) (`|GetArrayItem` _componenttags))
      (:`then`
        (return (`KismetArrayLibrary.Array_Contains` (`.MatchesWith_6_8802C2754F8795C67A4F4D9AE7154197` (break `/Game/DungeonGenerator/Data/ConnectionMatch` _returnvalue)) (`local.Connection`)))))))

(fn `CheckTileCondition`
  (returns (Return :type Boolean))
  (locals (ConditionMet :type Boolean :default false))
  (bind ((`TileCondition_25_38EFC60D4F3932C5CE1634AD03D78875` _tilecondition)) (break `/Game/DungeonGenerator/Data/TileData` (`self.TileData`)))
  (if (`KismetSystemLibrary.IsValidClass` _tilecondition)
    (bind _returnvalue (`|SpawnActorFromClass` _tilecondition (`self.GetTransform`) "AlwaysSpawn" "OverrideRootScale" null self (`self.DungeonGenerator`) null))
    (bind _return (`/Game/DungeonGenerator/Blueprints/TileCondition.CheckCondition` _returnvalue))
    (set `local.ConditionMet` _return)
    (`self.K2_DestroyActor` _returnvalue)
    (return (`local.ConditionMet`))
    (else
      (return true))))

(fn `CreateConnections`
  (locals (CurrentBox :type "BoxComponent Object Reference"))
  (`ActorComponent.K2_DestroyComponent` (`self.Connections`))
  (`KismetArrayLibrary.Array_Clear` (`self.Connections`))
  (for _array_element (`.Connections_6_45BF8D50405223D2E59948B062AA2031` (break `/Game/DungeonGenerator/Data/TileData` (`self.TileData`)))
    (bind ((`Transform_2_C1FF5E8344E708A538E5D9ADCC5696B7` _transform) (`Type_7_26122FC74EFF9E7F8E9B71B59A37741A` _type)) (break `/Game/DungeonGenerator/Data/TileConnection` _array_element))
    (bind _returnvalue (`AddComponent|NODE_AddBoxComponent-0` :`RelativeTransform` _transform))
    (set `local.CurrentBox` _returnvalue)
    (`KismetArrayLibrary.Array_AddUnique` (`/Game/DungeonGenerator/Blueprints/DungeonGenerator.UnfinishedConnections` (`self.DungeonGenerator`)) (`local.CurrentBox`))
    (`BoxComponent.SetBoxExtent` (`local.CurrentBox`) (`/Game/DungeonGenerator/Blueprints/DungeonGenerator.ConnectionQuerySize` (`self.DungeonGenerator`)) true)
    (set `ActorComponent.ComponentTags` (`|MakeArray` _type) (`local.CurrentBox`))
    (`KismetArrayLibrary.Array_Add` (`self.Connections`) (`local.CurrentBox`)))
  (return))

(fn `DestroyTile`
  (params (AfterLayout :type Boolean :default false))
  (`self.RemoveRemainingConnections`)
  (`/Engine/EditorBlueprintResources/StandardMacros.IsValid` (`self.Modifier`)
    (:`Is Valid`
      (`self.K2_DestroyActor` (`self.Modifier`)))
    (:`Is Not Valid`
      _))
  (if (`local.AfterLayout`)
    (`/Engine/EditorBlueprintResources/StandardMacros.DecrementInt` (`/Game/DungeonGenerator/Blueprints/DungeonGenerator.LayoutTilesSpawned` (`self.DungeonGenerator`))
      (:`  `
        _)))
  (`self.K2_DestroyActor`)
  (return))

(fn `RemoveRemainingConnections`
  (for _array_element (`self.Connections`)
    (`KismetArrayLibrary.Array_RemoveItem` (`/Game/DungeonGenerator/Blueprints/DungeonGenerator.UnfinishedConnections` (`self.DungeonGenerator`)) _array_element))
  (return))

(fn `RunChecks`
  (params (SkipChecks :type Boolean))
  (returns (Return :type Boolean))
  (if (`local.SkipChecks`)
    (`self.RemoveRemainingConnections`)
    (return true)
    (else
      (bind _isclear (`self.CheckCollision`))
      (if _isclear
        (bind _return (`self.CheckConnections`))
        (if _return
          (bind _return_2 (`self.CheckTileCondition`))
          (return _return_2)
          (else
            (return false)))
        (else
          (return false))))))

(fn `SetRow`
  (params (Row :type Name) (SpawnModifier :type Boolean))
  (bind _modifier (`self.Modifier`))
  (set `self.DataTableRow` Row)
  (`/Engine/EditorBlueprintResources/StandardMacros.IsValid` (`self.Modifier`)
    (:`Is Valid`
      (`self.K2_DestroyActor` (`self.Modifier`)))
    (:`Is Not Valid`
      _))
  (set `self.Modifier` null)
  (bind _returnvalue (`|GetDataTableRow` (`/Game/DungeonGenerator/Blueprints/DungeonGenerator.Tiles` (`self.DungeonGenerator`)) (`self.DataTableRow`))
    (:`then`
      (set `self.TileData` (`.TileData_3_9898053E4AEB04A7AD36ACA2E4DA45FC` (break `/Game/DungeonGenerator/Data/TileEntry` _returnvalue)))
      (`self.CreateConnections`)
      (`StaticMeshComponent.SetStaticMesh` (`self.CollisionMesh`) (`.CollisionMesh_10_595878D144A5E63942DFC5A4349024DE` (break `/Game/DungeonGenerator/Data/TileData` (`self.TileData`))))
      (if (`local.SpawnModifier`)
        (`self.SpawnModifier`)
        (`/Engine/EditorBlueprintResources/StandardMacros.IsValid` _modifier
          (:`Is Valid`
            (`/Game/DungeonGenerator/Blueprints/LayoutModifier.ModifyLayout` _modifier)))))))

(fn `SpawnAssociatedLevel`
  (returns (Level :type "LevelStreamingKismet Object Reference"))
  (bind (_returnvalue_location _returnvalue_rotation) (`KismetMathLibrary.BreakTransform` (`self.GetTransform`)))
  (bind (_boutsuccess _returnvalue) (`LevelStreamingKismet.LoadLevelInstance` (`.Map_2_6871C05D4C41DBC201A03D8195C1B201` (break `/Game/DungeonGenerator/Data/TileData` (`self.TileData`))) _returnvalue_location _returnvalue_rotation))
  (if _boutsuccess
    (return _returnvalue)
    (else
      (`KismetSystemLibrary.PrintString` (`KismetStringLibrary.Concat_StrStr` "Level for Table Row \"" (`KismetStringLibrary.Conv_NameToString` (`self.DataTableRow`)) "\" not found!") true true (struct :`R` 1.0 :`A` 1.0) 10.0))))

(fn `SpawnModifier`
  (bind ((`LayoutModifier_26_9460731241EBE507DA25C18F6C51A3DE` _layoutmodifier)) (break `/Game/DungeonGenerator/Data/TileData` (`self.TileData`)))
  (if (`KismetSystemLibrary.IsValidClass` _layoutmodifier)
    (bind _returnvalue (`|SpawnActorFromClass` _layoutmodifier (`self.GetTransform`) "AlwaysSpawn" "OverrideRootScale" null self (`self.DungeonGenerator`) null))
    (set `self.Modifier` _returnvalue)))

(fn `UserConstructionScript`
  (`self.SetRow` (`self.DataTableRow`)))