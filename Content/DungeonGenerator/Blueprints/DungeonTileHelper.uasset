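; Editor-time helper actor that records a dungeon tile level's data for the dungeon generator and destroys itself on BeginPlay.
; Its construction script resets the actor transform and fills TileData with the map path, built from a prefix and the current level name.
; It gathers every TileConnection actor's transform, type and DontStartHere flag into TileData's connections.
; The TileData collision mesh is shown on its StaticMesh, with visibility toggled by ShowCollisionMesh.
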(event `self.ReceiveBeginPlay`
  (`self.K2_DestroyActor`))

(fn `UserConstructionScript`
  (locals (Connections :type "Array of /Game/DungeonGenerator/Data/TileConnection Structure"))
  (`self.K2_SetActorTransform` (`KismetMathLibrary.MakeTransform` (0.0 0.0 0.0)))
  (`SceneComponent.SetVisibility` (`self.StaticMesh`) (`self.ShowCollisionMesh`) false)
  (bind _returnvalue (`GameplayStatics.GetCurrentLevelName` false))
  (setmembers `/Game/DungeonGenerator/Data/TileData` :`StructRef` (`self.TileData`) :`Map` (`KismetStringLibrary.Concat_StrStr` (`self.MapPathPrefix`) _returnvalue))
  (bind _outactors (`GameplayStatics.GetAllActorsOfClass` "/Game/DungeonGenerator/Blueprints/TileConnection.TileConnection_C"))
  (for _array_element _outactors
    (`KismetArrayLibrary.Array_Add` (`local.Connections`) (make `/Game/DungeonGenerator/Data/TileConnection` (`self.GetTransform` _array_element) (`/Game/DungeonGenerator/Blueprints/TileConnection.ConnectionType` _array_element) (`/Game/DungeonGenerator/Blueprints/TileConnection.DontStartHere` _array_element))))
  (bind _structout (setmembers `/Game/DungeonGenerator/Data/TileData` :`StructRef` (`self.TileData`) :`Connections` (`local.Connections`)))
  (`StaticMeshComponent.SetStaticMesh` (`self.StaticMesh`) (`.CollisionMesh_10_595878D144A5E63942DFC5A4349024DE` (break `/Game/DungeonGenerator/Data/TileData` _structout))))