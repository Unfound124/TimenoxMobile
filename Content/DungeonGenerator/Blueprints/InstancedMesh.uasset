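; InstancedMesh is a placeholder actor that hands its mesh over to the dungeon generator at runtime.
; The construction script applies the configured StaticMesh to TheMesh component.
; On BeginPlay it finds the first DungeonGenerator, passes TheMesh to AddInstancedMesh, then destroys itself.
; If no generator exists, the actor stays in the level unchanged.
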(event `self.ReceiveBeginPlay`
  (bind _outactors (`GameplayStatics.GetAllActorsOfClass` "/Game/DungeonGenerator/Blueprints/DungeonGenerator.DungeonGenerator_C"))
  (if (`KismetArrayLibrary.Array_IsValidIndex` _outactors)
    (`/Game/DungeonGenerator/Blueprints/DungeonGenerator.AddInstancedMesh` (`|GetArrayItem` _outactors) (`self.TheMesh`))
    (`self.K2_DestroyActor`)))

(fn `UserConstructionScript`
  (`StaticMeshComponent.SetStaticMesh` (`self.TheMesh`) (`self.StaticMesh`)))