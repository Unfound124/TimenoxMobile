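; MapBounds is a dungeon generator actor that forms a box-shaped boundary from six box components around an area defined by its Size variable.
; Its construction script places each of the Top, Bottom, Front, Back, Left and Right boxes just outside the matching face.
; Each box is a fixed-thickness slab sized to cover its face, so the inner volume matches Size exactly.
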(fn `UserConstructionScript`
  (bind (_size_x _size_y _size_z) (`KismetMathLibrary.BreakVector` (`self.Size`)))
  (bind _bottom (`self.Bottom`))
  (bind _top (`self.Top`))
  (bind _front (`self.Front`))
  (bind _back (`self.Back`))
  (bind _left (`self.Left`))
  (bind _right (`self.Right`))
  (bind _returnvalue (/ _size_y 2.0))
  (bind _returnvalue_2 (/ _size_x 2.0))
  (bind _returnvalue_3 (/ _size_z 2.0))
  (bind _returnvalue_4 (+ _returnvalue_2 50.0))
  (bind _returnvalue_5 (+ _returnvalue_3 50.0))
  (bind _returnvalue_6 (+ _returnvalue 50.0))
  (`|ExecutionSequence`
    (:`then_0`
      (`SceneComponent.K2_SetRelativeLocation` _bottom (`KismetMathLibrary.MakeVector` 0.0 0.0 (- 0.0 _returnvalue_5)) false false)
      (`BoxComponent.SetBoxExtent` _bottom (`KismetMathLibrary.MakeVector` _returnvalue_2 _returnvalue 50.0) true))
    (:`then_1`
      (`SceneComponent.K2_SetRelativeLocation` _top (`KismetMathLibrary.MakeVector` 0.0 0.0 _returnvalue_5) false false)
      (`BoxComponent.SetBoxExtent` _top (`KismetMathLibrary.MakeVector` _returnvalue_2 _returnvalue 50.0) true))
    (:`then_2`
      (`SceneComponent.K2_SetRelativeLocation` _front (`KismetMathLibrary.MakeVector` _returnvalue_4) false false)
      (`BoxComponent.SetBoxExtent` _front (`KismetMathLibrary.MakeVector` 50.0 _returnvalue _returnvalue_3) true))
    (:`then_3`
      (`SceneComponent.K2_SetRelativeLocation` _back (`KismetMathLibrary.MakeVector` (- 0.0 _returnvalue_4)) false false)
      (`BoxComponent.SetBoxExtent` _back (`KismetMathLibrary.MakeVector` 50.0 _returnvalue _returnvalue_3) true))
    (:`then_4`
      (`SceneComponent.K2_SetRelativeLocation` _left (`KismetMathLibrary.MakeVector` 0.0 (- 0.0 _returnvalue_6)) false false)
      (`BoxComponent.SetBoxExtent` _left (`KismetMathLibrary.MakeVector` _returnvalue_2 50.0 _returnvalue_3) true))
    (:`then_5`
      (`SceneComponent.K2_SetRelativeLocation` _right (`KismetMathLibrary.MakeVector` 0.0 _returnvalue_6) false false)
      (`BoxComponent.SetBoxExtent` _right (`KismetMathLibrary.MakeVector` _returnvalue_2 50.0 _returnvalue_3) true))))