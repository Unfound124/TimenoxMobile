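; Player pawn for Timenox: moves by touch or virtual joystick, with time running at full speed during input and slowing sharply when idle.
; Tick aims the barrel at the closest turret from a sphere trace and fires projectiles, throttled by a Delay; without a target, aim follows input.
; The game instance's InputMethod selects controls; touch gates movement toward the finger and shows a reticle.
; Death disables input, hides the mesh and slows time.
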(event `TargetEnemy`
  (bind _playerbarrel (`self.PlayerBarrel`))
  (bind (_returnvalue_roll _returnvalue_pitch _returnvalue_yaw) (`KismetMathLibrary.BreakRotator` (`KismetMathLibrary.MakeRotationFromAxes` (`KismetMathLibrary.MakeVector` (* (`self.GetInputAxisValue`) -1.0) (`self.GetInputAxisValue`)))))
  (bind (_returnvalue_roll_2 _returnvalue_pitch_2 _returnvalue_yaw_2) (`KismetMathLibrary.BreakRotator` (`KismetMathLibrary.FindLookAtRotation` (`SceneComponent.K2_GetComponentLocation` (`self.PlayerBarrel`)) (`.Location` (`GameplayStatics.BreakHitResult` (`PlayerController.GetHitResultUnderFingerByChannel` (`GameplayStatics.GetPlayerController` 0) "Touch1" "TraceTypeQuery1" true))))))
  (bind _turretobject (`self.getClosestTurret`))
  (`/Engine/EditorBlueprintResources/StandardMacros.IsValid` _turretobject
    (:`Is Valid`
      (bind (_returnvalue_roll_3 _returnvalue_pitch_3 _returnvalue_yaw_3) (`KismetMathLibrary.BreakRotator` (`KismetMathLibrary.FindLookAtRotation` (`SceneComponent.K2_GetComponentLocation` _playerbarrel) (`self.K2_GetActorLocation` _turretobject))))
      (`SceneComponent.K2_SetWorldRotation` _playerbarrel (`KismetMathLibrary.MakeRotator` 0.0 0.0 (+ _returnvalue_yaw_3 180.0)) false false)
      (`self.Shoot`))
    (:`Is Not Valid`
      (`SceneComponent.K2_SetWorldRotation` (`self.PlayerBarrel`) (`KismetMathLibrary.MakeRotator` 0.0 0.0 (+ (select `/Game/InputMethod` (`/Game/GI_Timenox.InputMethod` (cast `/Game/GI_Timenox` (`GameplayStatics.GetGameInstance`) :!pure true)) :`NewEnumerator2` _returnvalue_yaw_2 :`NewEnumerator0` _returnvalue_yaw_2 :`NewEnumerator1` (+ _returnvalue_yaw -90.0)) 180.0)) false false))))

(event `Shoot`
  (`KismetSystemLibrary.Delay` (`self.PlayerFireRate`))
  (`|SpawnActorFromClass` "/Game/Player/PlayerProjectile.PlayerProjectile_C" (`SceneComponent.K2_GetComponentToWorld` (`self.Muzzle`)) "Undefined" "OverrideRootScale" null (`self.ProjectileSpeed`) null))

(event `self.ReceiveBeginPlay`
  (`KismetSystemLibrary.Delay` 0.1)
  (`self.UpdateInputMode`)
  (bind _returnvalue (`|CreateWidget` "/Game/Widgets/Reticle.Reticle_C"))
  (set `self.ReticleRef` _returnvalue))

(event `UpdateInputMode`
  (bind _returnvalue (`GameplayStatics.GetPlayerController` 0))
  (`PlayerController.ActivateTouchInterface` _returnvalue (select `/Game/InputMethod` (`/Game/GI_Timenox.InputMethod` (cast `/Game/GI_Timenox` (`GameplayStatics.GetGameInstance`) :!pure true)) :`NewEnumerator1` "/Game/TouchInterface/TimenoxTouchInterface.TimenoxTouchInterface" :!type "TouchInterface Object Reference"))
  (`PlayerController.SetVirtualJoystickVisibility` _returnvalue true))

(event `Die`
  (`self.DisableInput` (`GameplayStatics.GetPlayerController` 0))
  (`SceneComponent.SetVisibility` (`self.Cube`) false true)
  (`GameplayStatics.SetGlobalTimeDilation` 0.05))

(event `self.ReceiveTick`
  (params (DeltaSeconds :type "Float (single-precision)"))
  (bind (_returnvalue_x _returnvalue_y) (`KismetMathLibrary.BreakVector` (`self.K2_GetActorLocation`)))
  (bind _returnvalue (`GameplayStatics.GetPlayerController` 0))
  (bind _reticleref (`self.ReticleRef`))
  (bind (_bblockinghit _binitialoverlap _time _distance _location) (`GameplayStatics.BreakHitResult` (`PlayerController.GetHitResultUnderFingerByChannel` _returnvalue "Touch1" "TraceTypeQuery1" true)))
  (`self.TargetEnemy`)
  (switch `/Game/InputMethod` (`/Game/GI_Timenox.InputMethod` (cast `/Game/GI_Timenox` (`GameplayStatics.GetGameInstance`) :!pure true))
    (:`NewEnumerator0`
      (`/Engine/EditorBlueprintResources/StandardMacros.Gate` true :!label _label
        (:`Exit`
          (`self.AddMovementInput` (`KismetMathLibrary.MakeVector` (- (.x _location) _returnvalue_x) (- (.y _location) _returnvalue_y)))
          (`/Engine/EditorBlueprintResources/StandardMacros.IsValid` _reticleref
            (:`Is Valid`
              (`UserWidget.SetPositionInViewport` _reticleref (`GameplayStatics.ProjectWorldToScreen` _returnvalue _location true) true))))))
    (:`NewEnumerator1`
      (if (and (== (`self.GetInputAxisValue`) 0.0) (== (`self.GetInputAxisValue`) 0.0))
        (`GameplayStatics.SetGlobalTimeDilation` 0.1 :!label _label_2)
        (else
          (`GameplayStatics.SetGlobalTimeDilation` 1.0 :!label _label_3))))))

(event `EndTouch`
  (bind _reticleref (`self.ReticleRef`))
  (`|ExecutionSequence`
    (:`then_0`
      (`/Engine/EditorBlueprintResources/StandardMacros.IsValid` _reticleref
        (:`Is Valid`
          (`Widget.RemoveFromParent` _reticleref))))
    (:`then_1`
      (goto _label_2))))

(event `TriggerTouch`
  (bind _reticleref (`self.ReticleRef`))
  (`|ExecutionSequence`
    (:`then_0`
      (if (`|EnumEquality` (`/Game/GI_Timenox.InputMethod` (cast `/Game/GI_Timenox` (`GameplayStatics.GetGameInstance`) :!pure true)) "NewEnumerator0")
        (`/Engine/EditorBlueprintResources/StandardMacros.IsValid` _reticleref
          (:`Is Valid`
            (`UserWidget.AddToViewport` _reticleref 0)))))
    (:`then_1`
      (goto _label_3))))

(event `InputTouch`
  (params (Location :type "Vector Structure") (FingerIndex :type "ETouchIndex Enum"))
  (:`Pressed`
    (`self.TriggerTouch`)
    (goto _label :!via `Open`))
  (:`Released`
    (`self.EndTouch`)
    (goto _label :!via `Close`)))

(event `InputAxis|MoveUp`
  (params (AxisValue :type "Float (single-precision)"))
  (switch `/Game/InputMethod` (`/Game/GI_Timenox.InputMethod` (cast `/Game/GI_Timenox` (`GameplayStatics.GetGameInstance`) :!pure true))
    (:`NewEnumerator1`
      (`self.AddMovementInput` (1.0 0.0 0.0) AxisValue))))

(event `InputAxis|MoveRight`
  (params (AxisValue :type "Float (single-precision)"))
  (switch `/Game/InputMethod` (`/Game/GI_Timenox.InputMethod` (cast `/Game/GI_Timenox` (`GameplayStatics.GetGameInstance`) :!pure true))
    (:`NewEnumerator1`
      (`self.AddMovementInput` (0.0 1.0 0.0) AxisValue))))

(fn `getClosestTurret`
  (returns (TurretObject :type "Actor Object Reference"))
  (locals (ReturnVal :type "HitResult Structure"))
  (bind _returnvalue (`self.K2_GetActorLocation`))
  (bind _returnval (`local.ReturnVal`))
  (bind (_outhits _returnvalue_2) (`KismetSystemLibrary.SphereTraceMultiForObjects` _returnvalue (+ _returnvalue (0.0 0.0 1.0)) 2000.0 (`|MakeArray` "ObjectTypeQuery8" :!type "EObjectTypeQuery Enum") false (`|MakeArray` null :!type "Actor Object Reference")))
  (if _returnvalue_2
    (set `local.ReturnVal` (`|GetArrayItem` _outhits))
    (for _array_element _outhits
      (set `local.ReturnVal` (select `bool` (<= (`.Distance` (`GameplayStatics.BreakHitResult` _array_element)) (`.Distance` (`GameplayStatics.BreakHitResult` _returnval))) :`false` _returnval :`true` _array_element)))
    (return (`ActorComponent.GetOwner` (`.HitComponent` (`GameplayStatics.BreakHitResult` (`local.ReturnVal`)))))
    (else
      (return null))))

(fn `UserConstructionScript`)